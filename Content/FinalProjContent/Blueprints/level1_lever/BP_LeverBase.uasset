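; BP_LeverBase is a level 1 lever mount whose base and lever are revealed in stages.
; BeginPlay hides both components, then after a 30-second delay shows the base and keeps the lever hidden.
; Any overlap with the Box spawns an emitter at the actor's location and unhides the lever, with no check on the overlapping actor or whether the delay has finished.
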(event OnComponentBeginOverlap(Box)
  (params (OverlappedComponent :type Primitive%20Component%20Object%20Reference) (OtherActor :type Actor%20Object%20Reference) (OtherComp :type Primitive%20Component%20Object%20Reference) (OtherBodyIndex :type Integer) (bFromSweep :type Boolean) (SweepResult :type Hit%20Result%20Structure%20%28by%20ref%29))
  ;[1 1 1] the lever appears after finding lever in map
  (Effects|SpawnEmitteratLocation 0 (Transformation|GetActorLocation))
  (Development|SetHiddeninGame (Variables|Default|GetLever) false false))

(event EventTick
  (params (DeltaSeconds :type Float%20%28single-precision%29)))

(event EventBeginPlay
  (bind _leverbase (Variables|Default|GetLeverBase))
  (bind _lever (Variables|Default|GetLever))
  ;[1 1 1] lever and base appear after level starts
  (Development|SetHiddeninGame _leverbase true false)
  (Development|SetHiddeninGame _lever true false)
  (Utilities|FlowControl|Delay 3e+01)
  (Development|SetHiddeninGame _leverbase false false)
  (Development|SetHiddeninGame _lever true false))

(fn ConstructionScript)